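; BP_GlobalWind is a placeable actor that sets global wind values for materials through the MPC_GlobalWind material parameter collection.
; Its GlobalWind function writes the WindSpeed and WindIntensity variables as scalar parameters and the Arrow component's forward vector as the wind direction.
; The function runs in the construction script and every Tick, so values update both when the actor is constructed and continuously during play.
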(event `self.ReceiveTick`
  (params (DeltaSeconds :type "Float (single-precision)"))
  (`self.GlobalWind`))

(fn `GlobalWind`
  (`KismetMaterialLibrary.SetScalarParameterValue` "/Game/Global_wind/MPC_GlobalWind.MPC_GlobalWind" "Wind_Speed" (`self.WindSpeed`))
  (`KismetMaterialLibrary.SetScalarParameterValue` "/Game/Global_wind/MPC_GlobalWind.MPC_GlobalWind" "Wind_Intensity" (`self.WindIntensity`))
  (`KismetMaterialLibrary.SetVectorParameterValue` "/Game/Global_wind/MPC_GlobalWind.MPC_GlobalWind" "Wind_Direction" (`KismetMathLibrary.Conv_VectorToLinearColor` (`SceneComponent.GetForwardVector` (`self.Arrow`)))))

(fn `UserConstructionScript`
  (`self.GlobalWind`))